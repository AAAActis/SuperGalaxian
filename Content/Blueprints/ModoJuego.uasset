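; ModoJuego is a game mode Blueprint that decides victory and defeat for a level.
; Tick checks the kill count against the win threshold to load Level2, and the player-death flag to reload Level1.
; BeginPlay runs a one-second looping Delay as a timer that also reloads Level1 after a minute.
; Each outcome prints a message, and this graph only reads the kill and death variables.
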(event EventTick
  (params (DeltaSeconds :type Float%20%28single-precision%29))
  (Utilities|FlowControl|Sequence
    (:then_0
      (if (>= (Variables|Default|GetMuertes) (Variables|Default|GetKillWin))
        (Development|PrintString "Has Ganado!")
        (Game|OpenLevel(byName) "Level2")))
    (:then_1
      (if (Variables|Default|GetMuerteJugador)
        (Development|PrintString "Derrota")
        (Game|OpenLevel(byName) "Level1")))))

(event EventBeginPlay
  (Utilities|FlowControl|Sequence
    (:then_0
      (Utilities|FlowControl|Delay 1.0 :!label _label)
      (Variables|Default|Settiempo (+ (Variables|Default|Gettiempo) 1.0))
      (if (>= (Variables|Default|Gettiempo) 6e+01)
        (Development|PrintString "DERROTA")
        (Game|OpenLevel(byName) "Level1")
        (else
          (goto _label))))))

(fn ConstructionScript)