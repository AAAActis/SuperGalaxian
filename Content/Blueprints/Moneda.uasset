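; Moneda is a coin pickup that spins in place and awards points to the player.
; Tick applies a fixed local rotation each frame without delta time, so spin speed depends on frame rate.
; On overlap with a Jugador, it adds two points to Puntaje in the ModoJuego game mode, prints the new score and destroys itself.
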(event Collision|EventActorBeginOverlap
  (params (OtherActor :type Actor%20Object%20Reference))
  (bind _asjugador (Utilities|Casting|CastToJugador OtherActor))
  (Variables|Default|Setjugador _asjugador)
  (bind _asmodo_juego (Utilities|Casting|CastToModoJuego (Game|GetGameMode)))
  (bind _output_get (Variables|/Game/Blueprints/ModoJuego.ModoJuego_C|Setpuntaje _asmodo_juego (+ (Variables|/Game/Blueprints/ModoJuego.ModoJuego_C|Getpuntaje _asmodo_juego) 2)))
  (Development|PrintString (Utilities|String|ToString(Integer) _output_get))
  (Actor|DestroyActor))

(event EventTick
  (params (DeltaSeconds :type Float%20%28single-precision%29))
  (Transformation|AddActorLocalRotation "0,-1.000000, 0" false false))

(fn ConstructionScript)