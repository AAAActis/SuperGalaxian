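; Curador is a healing actor that restores the health of a Jugador when it overlaps it.
; The overlap event casts the other actor to Jugador, stores the reference, and adds a fixed amount to VidaJugador at or below a threshold, otherwise setting it to VidaMaxima.
; The additive branch does not clamp to the maximum, and both branches print the new health.
; The actor stays in place afterwards, so each new overlap heals again.
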(event Collision|EventActorBeginOverlap
  (params (OtherActor :type Actor%20Object%20Reference))
  (bind _asjugador (Utilities|Casting|CastToJugador OtherActor))
  (Variables|Default|SetJugador _asjugador)
  (if (<= (Variables|/Game/Blueprints/Jugador.Jugador_C|GetvidaJugador (Variables|Default|GetJugador)) 5e+01)
    (bind _output_get (Variables|/Game/Blueprints/Jugador.Jugador_C|SetvidaJugador (Variables|Default|GetJugador) (+ (Variables|/Game/Blueprints/Jugador.Jugador_C|GetvidaJugador (Variables|Default|GetJugador)) 1e+02)))
    (Development|PrintString (Utilities|String|ToString(Float) _output_get))
    (else
      (bind _output_get_2 (Variables|/Game/Blueprints/Jugador.Jugador_C|SetvidaJugador (Variables|Default|GetJugador) (Variables|/Game/Blueprints/Jugador.Jugador_C|GetvidaMaxima (Variables|Default|GetJugador))))
      (Development|PrintString (Utilities|String|ToString(Float) _output_get_2)))))

(fn ConstructionScript)