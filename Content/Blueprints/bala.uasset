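; Bullet (bala) projectile actor that damages Enemigo actors it overlaps.
; Each Tick it moves along its local X axis by a fixed, swept offset that is not scaled by delta time.
; A Delay on the same Tick chain destroys it after about one second.
; An overlap with an Enemigo subtracts one from VidaEnemigo and prints the result, without destroying the bullet.
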(event Collision|EventActorBeginOverlap
  (params (OtherActor :type Actor%20Object%20Reference))
  (bind _asenemigo (Utilities|Casting|CastToEnemigo OtherActor))
  (bind _output_get (Variables|Default|SetEnemigo _asenemigo))
  (bind _output_get_2 (Variables|/Game/Blueprints/Enemigo.Enemigo_C|SetvidaEnemigo _output_get (- (Variables|/Game/Blueprints/Enemigo.Enemigo_C|GetvidaEnemigo _output_get) 1.0)))
  (Development|PrintString (Utilities|String|ToString(Float) _output_get_2)))

(event EventTick
  (params (DeltaSeconds :type Float%20%28single-precision%29))
  (Transformation|AddActorLocalOffset "90.000000, 0, 0" true false)
  (Utilities|FlowControl|Delay 1.0)
  (Actor|DestroyActor))

(fn ConstructionScript)