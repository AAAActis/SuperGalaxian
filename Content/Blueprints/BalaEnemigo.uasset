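; BalaEnemigo is an enemy bullet Blueprint that costs the player a life on contact.
; Tick moves it a fixed step along negative local X each frame, unscaled by delta time, and a Delay destroys it after five seconds.
; Overlapping a Jugador decrements VidasJugador, prints the remaining lives and destroys the bullet, while other actors are ignored.
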(event EventTick
  (params (DeltaSeconds :type Float%20%28single-precision%29))
  (Transformation|AddActorLocalOffset "-50.000000, 0, 0" false false)
  (Utilities|FlowControl|Delay 5.0)
  (Actor|DestroyActor))

(event Collision|EventActorBeginOverlap
  (params (OtherActor :type Actor%20Object%20Reference))
  (bind _asjugador (Utilities|Casting|CastToJugador OtherActor))
  (bind _output_get (Variables|Default|SetJugador _asjugador))
  (bind _output_get_2 (Variables|/Game/Blueprints/Jugador.Jugador_C|SetVidasJugador _output_get (- (Variables|/Game/Blueprints/Jugador.Jugador_C|GetVidasJugador _output_get) 1.0)))
  (Development|PrintString (Utilities|String|ToString(Float) _output_get_2))
  (Actor|DestroyActor))

(fn ConstructionScript)