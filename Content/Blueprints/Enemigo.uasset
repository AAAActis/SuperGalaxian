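; Enemy actor that sways sideways, makes attack runs firing BalaEnemigo, and dies when VidaEnemigo runs out.
; Tick applies per-frame swept offsets; EmpiezaAtaque adds forward motion along negative X, randomly delayed shots and randomly timed side switching.
; EmpiezaAtaque and TerminaAtaque drive EnemigoAtacando, whose inverse sets EnemigoPuedeAtacar; BeginPlay's one-second sway toggle loop starts only if already attacking.
; Death plays a sound, destroys the actor and increments ModoJuego's Muertes.
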(event EventBeginPlay
  (Utilities|FlowControl|Sequence
    (:then_0
      (if (Variables|Default|GetEnemigoAtacando)
        (Utilities|FlowControl|Delay 1.0 :!label _label)
        (if (Variables|Default|GetMoverALosCostados)
          (Variables|Default|SetMoverALosCostados false)
          (goto _label)
          (else
            (Variables|Default|SetMoverALosCostados true)
            (goto _label)))))
    (:then_2
      (Variables|Default|Setlocacion (Transformation|GetActorLocation)))))

(event EventTick
  (params (DeltaSeconds :type Float%20%28single-precision%29))
  (Utilities|FlowControl|Sequence
    (:then_0
      (if (Variables|Default|GetEmpiezaAtaque)
        (Utilities|FlowControl|Sequence
          (:then_0
            (Transformation|AddActorLocalOffset "-15.000000,0.000000, 0" true false)
            (Utilities|FlowControl|Delay (Math|Random|RandomFloatinRange 1.0 2.5))
            (Game|SpawnActorfromClass "/Game/Blueprints/BalaEnemigo.BalaEnemigo_C" (Transformation|GetActorTransform) "Undefined" 0 0))
          (:then_1
            (if (Variables|Default|GetMoverCostadoAtaque)
              (Transformation|AddActorLocalOffset (Math|Vector|MakeVector 0.0 (* (Variables|Default|GetVelocidadAtaque) 1.0) 0.0) true false)
              (else
                (Transformation|AddActorLocalOffset (Math|Vector|MakeVector 0.0 (* (Variables|Default|GetVelocidadAtaque) -1.0) 0.0) true false))))
          (:then_2
            (Utilities|FlowControl|Delay (Math|Random|RandomFloatinRange 1.0 2.6) :!label _label)
            (if (Variables|Default|GetMoverCostadoAtaque)
              (Variables|Default|SetMoverCostadoAtaque false)
              (goto _label)
              (else
                (Variables|Default|SetMoverCostadoAtaque true)
                (goto _label)))))))
    (:then_1
      (if (Variables|Default|GetEmpiezaAtaque)
        (Variables|Default|SetEnemigoAtacando true)))
    (:then_2
      (if (Variables|Default|GetTerminaAtaque)
        (Variables|Default|SetEnemigoAtacando false)))
    (:then_3
      (if (Variables|Default|GetMoverALosCostados)
        (Transformation|AddActorLocalOffset (Math|Vector|MakeVector 0.0 (* (Variables|Default|GetVelocidad) 1.0) 0.0) true false)
        (else
          (Transformation|AddActorLocalOffset (Math|Vector|MakeVector 0.0 (* (Variables|Default|GetVelocidad) -1.0) 0.0) true false))))
    (:then_4
      (if (<= (Variables|Default|GetvidaEnemigo) 0.0)
        (Utilities|FlowControl|Sequence
          (:then_0
            (Audio|PlaySoundatLocation "/Game/Sonidos/Bomba.Bomba" "0, 0, 0" "0, 0, 0" 1.0 1.0 0.0 0 0 0))
          (:then_1
            (Actor|DestroyActor)
            (bind _asmodo_juego (Utilities|Casting|CastToModoJuego (Game|GetGameMode)))
            (bind _output_get (Variables|Default|SetModoJuego _asmodo_juego))
            (bind _output_get_2 (Variables|/Game/Blueprints/ModoJuego.ModoJuego_C|SetMuertes _output_get (+ (Variables|/Game/Blueprints/ModoJuego.ModoJuego_C|GetMuertes _output_get) 1)))
            (Development|PrintString (Utilities|String|ToString(Integer) _output_get_2))))))
    (:then_5
      (if (Variables|Default|GetEnemigoAtacando)
        (Variables|Default|SetEnemigoPuedeAtacar false)
        (else
          (Variables|Default|SetEnemigoPuedeAtacar true))))))

(fn ConstructionScript)